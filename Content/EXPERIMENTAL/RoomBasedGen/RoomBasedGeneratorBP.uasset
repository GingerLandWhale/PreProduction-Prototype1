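; Experimental room-based map generator Blueprint, currently an unfinished skeleton that produces no rooms.
; The NewSeedMap input press draws a random room variant from a random stream, gathers all RoomTemplate actors, then rolls one of eight directions from the same stream.
; A nested branch chain tests the direction, but every branch is empty and the gathered actors go unused.
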(event EventBeginPlay)

(event Collision|EventActorBeginOverlap
  (params (OtherActor :type Actor%20Object%20Reference)))

(event EventTick
  (params (DeltaSeconds :type Float%20%28single-precision%29)))

(event Input|ActionEvents|InputActionNewSeedMap
  (params (Key :type Key%20Structure :default "None"))
  (:Pressed
    (Variables|Default|SetRoomVar (Math|Random|RandomIntegerinRangefromStream 0 3 (Variables|Default|GetStream)))
    (Actor|GetAllActorsOfClass "/Game/EXPERIMENTAL/Rooms/RoomTemplate.RoomTemplate_C")
    (Variables|Default|SetDirection (Math|Random|RandomIntegerinRangefromStream 1 8 (Variables|Default|GetStream)))
    (if (not (== (Variables|Default|GetDirection) 1))
      (if (not (== (Variables|Default|GetDirection) 2))
        (if (not (== (Variables|Default|GetDirection) 3))
          (if (not (== (Variables|Default|GetDirection) 4))
            (if (not (== (Variables|Default|GetDirection) 5))
              (if (not (== (Variables|Default|GetDirection) 6))
                (if (not (== (Variables|Default|GetDirection) 7))
                  (if (== (Variables|Default|GetDirection) 8)
                    _))))))))))

(fn ConstructionScript)